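; Destructible wall actor that reacts to hits and breaks apart, judging by its name and projectile folder.
; Both component hits and fractures call PlayFX, which plays an explosion sound and spawns an emitter at the impact point.
; On fracture it also sets IsBroken, disables gravity, ignores pawns and physics bodies, applies a radial impulse from its center, then destroys itself after a short delay.
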(event OnComponentFracture(DestructibleComponent)
  (params (HitPoint :type Vector%20%28by%20ref%29 :default "0, 0, 0") (HitDirection :type Vector%20%28by%20ref%29 :default "0, 0, 0"))
  (bind _destructiblecomponent (Variables|Default|GetDestructibleComponent))
  (bind _returnvalue (Transformation|GetWorldLocation _destructiblecomponent))
  (CallFunction|PlayFX HitPoint)
  (Variables|Default|SetIsBroken true)
  (Physics|SetEnableGravity (Variables|Default|GetDestructibleComponent) false)
  (Collision|SetCollisionResponsetoChannel (Variables|Default|GetDestructibleComponent) "ECC_Pawn" "ECR_Ignore")
  (Collision|SetCollisionResponsetoChannel (Variables|Default|GetDestructibleComponent) "ECC_PhysicsBody" "ECR_Ignore")
  (Collision|SetCollisionResponsetoChannel (Variables|Default|GetDestructibleComponent) "ECC_WorldStatic" "ECR_Block")
  (Physics|AddRadialImpulse _destructiblecomponent (Math|Vector|MakeVector (.x _returnvalue) (.y _returnvalue) (.z _returnvalue)) 0.0 0.0 "RIF_Linear" false)
  (Utilities|FlowControl|Delay 0.2)
  (Actor|DestroyActor))

(event OnComponentHit(DestructibleComponent)
  (params (HitComponent :type Primitive%20Component%20Object%20Reference) (OtherActor :type Actor%20Object%20Reference) (OtherComp :type Primitive%20Component%20Object%20Reference) (NormalImpulse :type Vector :default "0, 0, 0") (Hit :type Hit%20Result%20Structure%20%28by%20ref%29))
  (CallFunction|PlayFX (.location Hit)))

(fn ConstructionScript)

(fn PlayFX
  (params (Location :type Vector))
  (Audio|PlaySound2D "/Game/StarterContent/Audio/Explosion_Cue.Explosion_Cue" 1.0 1.0 0.0 0 0)
  (Effects|SpawnEmitteratLocation 0 Location (Transformation|GetWorldRotation (Variables|Default|GetDestructibleComponent))))