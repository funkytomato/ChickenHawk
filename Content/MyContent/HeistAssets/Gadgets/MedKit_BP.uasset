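; MedKit_BP is a health pickup that adds HealAmount to the Health of an overlapping actor that passes a cast, unless Health is already 100.
; The pickup is consumed only when the heal reaches 100, where Health is clamped; smaller heals leave it active.
; On consumption, CanRespawn selects between destroying the actor and a Respawn event that hides the mesh and disables collision for RespawnTime.
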(event OnComponentBeginOverlap(PickupArea)
  (params (OverlappedComponent :type Primitive%20Component%20Object%20Reference) (OtherActor :type Actor%20Object%20Reference) (OtherComp :type Primitive%20Component%20Object%20Reference) (OtherBodyIndex :type Integer) (bFromSweep :type Boolean) (SweepResult :type Hit%20Result%20Structure%20%28by%20ref%29))
  (bind _asplayer_base (Utilities|Casting|CastTo OtherActor))
  (if (not (== (Variables|Default|GetHealth _asplayer_base) 1e+02))
    (bind _output_get (Variables|Default|SetHealth _asplayer_base (+ (Variables|Default|GetHealth _asplayer_base) (Variables|HealthKitStats|GetHealAmount))))
    (if (>= _output_get 1e+02)
      (Variables|Default|SetHealth _asplayer_base 1e+02)
      (if (Variables|HealthKitStats|GetCan%20Respawn?)
        (CallFunction|Respawn)
        (else
          (Actor|DestroyActor))))))

(event Custom|Respawn
  (Rendering|SetVisibility (Variables|Default|GetHealthKit) false false)
  (Collision|SetCollisionEnabled (Variables|Default|GetPickup%20Area) "NoCollision")
  (Utilities|FlowControl|Delay (Variables|HealthKitStats|GetRespawn%20Time))
  (Rendering|SetVisibility (Variables|Default|GetHealthKit) true false)
  (Collision|SetCollisionEnabled (Variables|Default|GetPickup%20Area) "QueryAndPhysics"))

(fn ConstructionScript)