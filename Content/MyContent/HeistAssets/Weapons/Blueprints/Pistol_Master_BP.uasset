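; Master pistol weapon Blueprint that handles the cosmetic effects of firing and reloading.
; FirePistol plays a sound and gunshot particle at the Muzzle socket, spawns an empty case actor at the Ejection Port socket, and plays a non-looping mesh animation.
; ReloadMagazine spawns a dropped magazine actor at the Magazine socket.
; The file contains no damage, projectile or ammo logic.
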(event Custom|Fire%20Pistol
  (bind _skeletalmesh (Variables|Default|GetSkeletalMesh))
  (bind _returnvalue (Transformation|GetSocketLocation _skeletalmesh "Muzzle"))
  (Audio|PlaySoundatLocation 0 _returnvalue "0, 0, 0" 1.0 1.0 0.0 0 0 0)
  (Effects|SpawnEmitteratLocation "/Game/PolygonHeist/ParticleFX/FX_Gunshot.FX_Gunshot" _returnvalue (Transformation|GetSocketRotation _skeletalmesh "Muzzle"))
  (Game|SpawnActorfromClass "/Game/MyContent/HeistAssets/Weapons/Pickups/Pistol_Empty_Case_BP.Pistol_Empty_Case_BP_C" (Transformation|GetSocketTransform _skeletalmesh "Ejection Port" "RTS_World") "Undefined" 0 0)
  (Components|Animation|PlayAnimation (Variables|Default|GetSkeletalMesh) 0 false))

(event Custom|Reload%20Magazine
  (Game|SpawnActorfromClass "/Game/MyContent/HeistAssets/Weapons/Pickups/Pistol_Mag_Drop_BP.Pistol_Mag_Drop_BP_C" (Transformation|GetSocketTransform (Variables|Default|GetSkeletalMesh) "Magazine" "RTS_World") "Undefined" 0 0))

(fn ConstructionScript)