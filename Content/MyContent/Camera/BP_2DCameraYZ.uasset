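; 2.5D side-scroller camera that follows MainTarget along Y and Z, with X distance driven by an interpolated zoom.
; Activation makes it the view target; each tick updates zoom, facing and look offsets, then eases the camera toward its computed position.
; While the target is in a camera volume, per-axis tracking modes choose that position from follow, set or volume values.
; Z also supports platform locking based on landing, height and falling.
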(event Custom|Activate
  ;[1 0.8659 0.4917 1 30] Set This Camera Active
  (Game|Player|SetViewTargetwithBlend (Game|GetPlayerController 0) self 0.0 "VTBlend_Linear" 0.0 false)
  (Variables|Default|SetCamZPos (+ (.Z (Math|Vector|BreakVector (Transformation|GetWorldLocation (Variables|/Script/Engine.Character|GetCapsuleComponent (Variables|Default|GetMainTarget))))) (/ (Variables|Default|GetZoom) 3.0))))

(event EventBeginPlay
  ;[1 0.8659 0.4917 1 30] Set This Camera Active
  (if (Variables|Bool|GetActive)
    (Game|Player|SetViewTargetwithBlend (Game|GetPlayerController 0) self 0.0 "VTBlend_Linear" 0.0 false)
    (Variables|Default|SetCamZPos (+ (.Z (Math|Vector|BreakVector (Transformation|GetWorldLocation (Variables|/Script/Engine.Character|GetCapsuleComponent (Variables|Default|GetMainTarget))))) (/ (Variables|Default|GetZoom) 3.0)))))

(event EventTick
  (params (DeltaSeconds :type Float%20%28single-precision%29))
  (bind (_zoom _y _returnvalue4 _returnvalue3) (Utilities|CalculateOffsets))
  ;[1 0.4177 0.8333 1 30] Camera Tick
  (Variables|Default|SetDelta DeltaSeconds)
  (CallFunction|Zooming)
  (CallFunction|FacingOffset)
  (CallFunction|UpdatePos)
  (CallFunction|LookOffest)
  (CallFunction|InVolumes)
  (if (Variables|Tracking|GetTracking)
    (Variables|Default|SetCamXPos _zoom)
    (CallFunction|YposOntrackType _y)
    (Utilities|ZposonTrackType _returnvalue4 _returnvalue3
      (:PlatfromLocked
        (bind (_returnvalue _returnvalue2) (CallFunction|PlatformLock))
        (CallFunction|LookingFunc _returnvalue _returnvalue2)))))

(fn ConstructionScript
  (bind _camera (Variables|Default|GetCamera))
  (bind _returnvalue (Transformation|GetWorldLocation _camera))
  (bind (_x _y) (Math|Vector|BreakVector _returnvalue))
  (Variables|Default|SetCamXPos _x)
  (Variables|Default|SetCamYPos _y))

(fn UpdatePos
  (bind _camera (Variables|Default|GetCamera))
  ;[1 0.44 0.6121 1 30] Y- left right, Z Up Down, X zoom. standard 2.5d
  (Transformation|SetWorldLocation _camera (Math|Interpolation|VInterpTo (Transformation|GetWorldLocation _camera) (Math|Vector|MakeVector (Variables|Default|GetCamXPos) (Variables|Default|GetCamYPos) (Variables|Default|GetCamZPos)) (Variables|Default|GetDelta) 7.0) false false))

(fn LookOffest
  (bind _maintarget (Variables|Default|GetMainTarget))
  (bind _cameracomponent (Variables|/Game/MyContent/Characters/Blueprints/HelicopterCharacterWithFixedJoystick.HelicopterCharacterWithFixedJoystick_C|GetCameraComponent _maintarget))
  (bind _lookoffset (Variables|/Game/CameraComponent.CameraComponent_C|GetLookOffset _cameracomponent))
  (if (or (Variables|/Game/CameraComponent.CameraComponent_C|GetLookUP _cameracomponent) (Variables|/Game/CameraComponent.CameraComponent_C|GetLookDown _cameracomponent))
    (Variables|offset|SetZLookOffset (Math|Interpolation|FInterpTo _lookoffset _lookoffset (Variables|Default|GetDelta) 0.01))
    (else
      (Variables|offset|SetZLookOffset (Math|Interpolation|FInterpTo (Variables|offset|GetZLookOffset) 0.0 (Variables|Default|GetDelta) 1e+01)))))

(fn YposOntrackType
  (params (FollowY :type Float%20%28single-precision%29))
  (switch Utilities|FlowControl|Switch|SwitchonEnum_TrackType (Variables|Tracking|GetYTrackingType)
    (:NewEnumerator1
      (Variables|Default|SetCamYPos FollowY))
    (:NewEnumerator2
      (Variables|Default|SetCamYPos FollowY))
    (:NewEnumerator0
      (Variables|Default|SetCamYPos (Variables|Default|GetVOLY)))
    (:NewEnumerator3
      (Variables|Default|SetCamYPos 0.0))
    (:NewEnumerator4
      (Development|PrintString "This Is not supported" true true "(R=1.000000,G=0.035352,B=0.000000,A=1.000000)"))))

(fn InVolumes
  (if (Variables|/Game/CameraComponent.CameraComponent_C|GetInCameraVolume (Variables|/Game/MyContent/Characters/Blueprints/HelicopterCharacterWithFixedJoystick.HelicopterCharacterWithFixedJoystick_C|GetCameraComponent (Variables|Default|GetMainTarget)))
    (Variables|Tracking|SetTracking true)
    (else
      (Variables|Tracking|SetTracking false))))

(fn LookingFunc
  (params (A :type Float%20%28single-precision%29) (CamZPos :type Float%20%28single-precision%29))
  (bind _maintarget (Variables|Default|GetMainTarget))
  (bind _cameracomponent (Variables|/Game/MyContent/Characters/Blueprints/HelicopterCharacterWithFixedJoystick.HelicopterCharacterWithFixedJoystick_C|GetCameraComponent _maintarget))
  (if (or (Variables|/Game/CameraComponent.CameraComponent_C|GetLookUP _cameracomponent) (Variables|/Game/CameraComponent.CameraComponent_C|GetLookDown _cameracomponent))
    (Variables|Default|SetCamZPos (+ A (Variables|offset|GetZLookOffset)))
    (Variables|Bool|SetLooking true)
    (elif (Variables|Bool|GetLooking)
      (Variables|Default|SetCamZPos CamZPos)
      (Variables|Bool|SetLooking false))))

(fn FacingOffset
  (Utilities|NewMacro0
    (:True
      (switch Utilities|FlowControl|Switch|SwitchonEnum_Faceing (Variables|/Game/CameraComponent.CameraComponent_C|GetFaceing (Variables|/Game/MyContent/Characters/Blueprints/HelicopterCharacterWithFixedJoystick.HelicopterCharacterWithFixedJoystick_C|GetCameraComponent (Variables|Default|GetMainTarget)))
        (:NewEnumerator0
          (Variables|offset|SetYOffset (Math|Interpolation|FInterpTo (Variables|offset|GetYOffset) 2e+02 (Variables|Default|GetDelta) 1.0)))
        (:NewEnumerator1
          (Variables|offset|SetYOffset (Math|Interpolation|FInterpTo (Variables|offset|GetYOffset) -2e+02 (Variables|Default|GetDelta) 1.0)))
        (:NewEnumerator3
          (Variables|offset|SetZOffset 0.0))))
    (:False
      (Variables|offset|SetYOffset (Math|Interpolation|FInterpTo (Variables|offset|GetYOffset) (Variables|offset|GetYOffset) (Variables|Default|GetDelta) 2.0)))))

(fn PlatformLock
  (bind _platlockoffest (Variables|Default|GetPlatLockOffest))
  (bind _maintarget (Variables|Default|GetMainTarget))
  (bind _delta (Variables|Default|GetDelta))
  (bind _zoom (Variables|Default|GetZoom))
  (bind _returnvalue (/ _zoom _platlockoffest))
  (bind _capsulecomponent (Variables|/Script/Engine.Character|GetCapsuleComponent _maintarget))
  (bind _returnvalue_2 (Transformation|GetWorldLocation _capsulecomponent))
  (bind _z (Math|Vector|BreakVector _returnvalue_2))
  (bind _returnvalue_3 (+ _z _returnvalue))
  (bind _returnvalue_4 (Math|Interpolation|FInterpTo _returnvalue_3 _returnvalue_3 _delta 1.0))
  (if (Math|Boolean|ORBoolean (Variables|/Game/MyContent/Characters/Blueprints/HelicopterCharacterWithFixedJoystick.HelicopterCharacterWithFixedJoystick_C|GetLanded _maintarget) (<= _returnvalue_3 (Variables|Default|GetCamZPos)) (and (>= _returnvalue_3 (Variables|Default|GetCamZPos)) (not (AI|Components|NavMovement|IsFalling (Variables|/Script/Engine.Character|GetCharacterMovement _maintarget)))))
    (Variables|Default|SetCamZPos _returnvalue_4)
    (else
      (return _returnvalue_3 _returnvalue_4))))

(fn Zooming
  (Variables|Default|SetZoom (Math|Interpolation|FInterpTo (Variables|Default|GetZoom) (Variables|Default|GetNewZoom) (Variables|Default|GetDelta) (Variables|Default|GetZoomSpeed))))