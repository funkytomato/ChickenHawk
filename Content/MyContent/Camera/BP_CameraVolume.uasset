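; BP_CameraVolume is a trigger volume that changes camera tracking and zoom when a player character enters it.
; Box overlaps respond to the helicopter character's CameraTracker component or any PaperCharacter, setting or clearing InVolume.
; On entry, Updatecamerainfo copies tracking types, zoom, zoom speed and fixed Y/Z values to CameraYZ or CameraPaper2D, chosen by CameraToUse.
; Box collision is briefly disabled at BeginPlay, then re-enabled after a short delay.
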(event OnComponentBeginOverlap(Box)
  (params (OverlappedComponent :type Primitive%20Component%20Object%20Reference) (OtherActor :type Actor%20Object%20Reference) (OtherComp :type Primitive%20Component%20Object%20Reference) (OtherBodyIndex :type Integer) (bFromSweep :type Boolean) (SweepResult :type Hit%20Result%20Structure%20%28by%20ref%29))
  ;[1 0.5526 0.7373] Detect if character has entered volume and setting appropriate tracking type
  (Utilities|FlowControl|Sequence
    (:then_0
      (bind _ashelicopter_character_with_fixed_joystick (Utilities|Casting|CastToHelicopterCharacterWithFixedJoystick OtherActor))
      (if (== (Variables|/Game/MyContent/Characters/Blueprints/HelicopterCharacterWithFixedJoystick.HelicopterCharacterWithFixedJoystick_C|GetCameraTracker _ashelicopter_character_with_fixed_joystick) OtherComp)
        (CallFunction|Updatecamerainfo)))
    (:then_1
      (Utilities|Casting|CastToPaperCharacter OtherActor)
      (CallFunction|Updatecamerainfo))))

(event OnComponentEndOverlap(Box)
  (params (OverlappedComponent :type Primitive%20Component%20Object%20Reference) (OtherActor :type Actor%20Object%20Reference) (OtherComp :type Primitive%20Component%20Object%20Reference) (OtherBodyIndex :type Integer))
  ;[1 0.5526 0.7373] Detect if character exit volume
  (Utilities|FlowControl|Sequence
    (:then_0
      (bind _ashelicopter_character_with_fixed_joystick (Utilities|Casting|CastToHelicopterCharacterWithFixedJoystick OtherActor))
      (if (== (Variables|/Game/MyContent/Characters/Blueprints/HelicopterCharacterWithFixedJoystick.HelicopterCharacterWithFixedJoystick_C|GetCameraTracker _ashelicopter_character_with_fixed_joystick) OtherComp)
        (Variables|Default|SetInVolume false :!label _label)))
    (:then_1
      (Utilities|Casting|CastToPaperCharacter OtherActor)
      (goto _label))))

(event EventBeginPlay
  (Collision|SetCollisionEnabled (Variables|Default|GetBox) "NoCollision")
  (Utilities|FlowControl|Delay 0.01)
  (Collision|SetCollisionEnabled (Variables|Default|GetBox) "QueryAndPhysics"))

(fn ConstructionScript)

(fn Updatecamerainfo
  (bind _camerapaper2d (Variables|CameraTypes|GetCameraPaper2D))
  (bind _zoomdistance (Variables|Default|GetZoomDistance))
  (bind _sety (Variables|Default|GetSETY))
  (bind _tracktypey (Variables|Default|GetTrackTypeY))
  (bind _tracktypez (Variables|Default|GetTrackTypeZ))
  (bind _setz (Variables|Default|GetSETZ))
  (bind _camerayz (Variables|CameraTypes|GetCameraYZ))
  (Variables|Default|SetInVolume true)
  (switch Utilities|FlowControl|Switch|SwitchonEnum_Perspective (Variables|CameraTypes|GetCameraToUse)
    (:NewEnumerator0
      (Variables|/Game/Camera2D/Blueprints/CameraMain/BP_2DCameraYZ.BP_2DCameraYZ_C|SetYTrackingType _camerayz _tracktypey)
      (Variables|/Game/Camera2D/Blueprints/CameraMain/BP_2DCameraYZ.BP_2DCameraYZ_C|SetZTrackingType _camerayz _tracktypez)
      (Variables|/Game/Camera2D/Blueprints/CameraMain/BP_2DCameraYZ.BP_2DCameraYZ_C|SetNewZoom _camerayz _zoomdistance)
      (Variables|/Game/Camera2D/Blueprints/CameraMain/BP_2DCameraYZ.BP_2DCameraYZ_C|SetVOLY _camerayz _sety)
      (Variables|/Game/Camera2D/Blueprints/CameraMain/BP_2DCameraYZ.BP_2DCameraYZ_C|SetVOLZ _camerayz _setz)
      (Variables|/Game/Camera2D/Blueprints/CameraMain/BP_2DCameraYZ.BP_2DCameraYZ_C|SetZoomSpeed _camerayz (Variables|Default|GetZoomSpeed)))
    (:NewEnumerator8
      (Variables|/Game/Camera2D/Blueprints/CameraMain/BP_Paper2DCamera.BP_Paper2DCamera_C|SetYTrackingType _camerapaper2d _tracktypey)
      (Variables|/Game/Camera2D/Blueprints/CameraMain/BP_Paper2DCamera.BP_Paper2DCamera_C|SetZTrackingType _camerapaper2d _tracktypez)
      (Variables|/Game/Camera2D/Blueprints/CameraMain/BP_Paper2DCamera.BP_Paper2DCamera_C|SetNewZoom _camerapaper2d _zoomdistance)
      (Variables|/Game/Camera2D/Blueprints/CameraMain/BP_Paper2DCamera.BP_Paper2DCamera_C|SetVOLY _camerapaper2d _sety)
      (Variables|/Game/Camera2D/Blueprints/CameraMain/BP_Paper2DCamera.BP_Paper2DCamera_C|SetVOLZ _camerapaper2d _setz)
      (Variables|/Game/Camera2D/Blueprints/CameraMain/BP_Paper2DCamera.BP_Paper2DCamera_C|SetZoomSpeed _camerapaper2d (Variables|Default|GetZoomSpeed)))))