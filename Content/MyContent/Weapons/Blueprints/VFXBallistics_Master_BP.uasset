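; First-person character master Blueprint for a ballistics VFX weapon setup: rifle, pistol, high-powered rifle, thrown grenade and right-click grenade launcher.
; A gated macro regulates fire rate and spam clicks, then a camera trace aims bullets from the muzzle at the crosshair target.
; Recoil is none, timeline-driven camera kick or growing cone spread.
; Muzzle smoke waits for trigger release to limit FX, and F traces for interaction.
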(event Custom|ChangeWeapon)

(event Custom|AimOffsetTrigger
  ;[1 1 1] Aim Offset
  (Utilities|AimOffsetTrace (Variables|MyCharacter|GetFirstPersonCamera) (Variables|AimOffset|GetAimOffsetMaxRange) (Variables|Default|GetProjectileSpawnPoint)))

(event Custom|ConeRecoil
  (bind _recoilconepershotadd (Variables|ConeRecoil|GetRecoilConePerShotAdd))
  ;[1 1 1] Cone Recoil Simple Example
  (bind _recoilconefloat (Timeline|ConeRecoilFloat PlayFromStart)
    (:Update
      (Variables|ConeRecoil|SetRecoilFloatSet _recoilconefloat)
      (Variables|ConeRecoil|SetConeRecoilYaw (* (Math|Float|Clamp(Float) (+ _recoilconepershotadd (Variables|ConeRecoil|GetConeRecoilYaw)) 0.0 (Variables|ConeRecoil|GetConeRecoilYawMAX)) _recoilconefloat))
      (Variables|ConeRecoil|SetConeRecoilPitch (* (Math|Float|Clamp(Float) (+ _recoilconepershotadd (Variables|ConeRecoil|GetConeRecoilPitch)) 0.0 (Variables|ConeRecoil|GetConeRecoilPitch%20MAX)) _recoilconefloat)))))

(event Custom|TriggerOFF
  ;[0.2075 0.4327 1] Activate Muzzle Smoke FX once trigger is lifted (we don't want to spawn too many smoke FX during rapid fire)
  (Components|Activation|Activate (Variables|Default|GetMuzzle_Smoke_light) false))

(event Custom|TriggerON
  ;[0.2075 0.4327 1] Activate Muzzle Smoke FX once trigger is lifted (we don't want to spawn too many smoke FX during rapid fire)
  (CallFunction|MuzzleSmokeOff))

(event Custom|MuzzleSmokeOff
  ;[0.2075 0.4327 1] MUZZLE SMOKE OFF
  (Components|Activation|Deactivate (Variables|Default|GetMuzzle_Smoke_light)))

(event EventTick
  (params (DeltaSeconds :type Float%20%28single-precision%29))
  ;[1 1 1] Movement Check Each Tick
  (if (>= (Math|Vector|VectorLength (Variables|/Script/Engine.MovementComponent|GetVelocity (Variables|Character|GetCharacterMovement))) 8e+02)
    (Variables|Default|SetCharacterMoving true)
    ;[0.2075 0.4327 1] Deactivate Muzzle Smoke On Movement Threshold
    (if (Components|Activation|IsActive (Variables|Default|GetMuzzle_Smoke_light)) :!label _label
      (CallFunction|MuzzleSmokeOff))
    (else
      (Variables|Default|SetCharacterMoving false)
      (if (Variables|Default|GetTriggerPressed)
        (goto _label)))))

(event EventBeginPlay
  ;[1 1 1] Set Gun Loc
  (Transformation|SetRelativeLocationAndRotation (Variables|MyCharacter|GetMesh2P) "-0.000032,-0.000121,-156.681747" "0,-10.000000, 0" false false)
  (Development|ExecuteConsoleCommand (Utilities|String|Append "r.Decal.FadeScreenSizeMult " (Utilities|String|ToString(Float) (Variables|Default|GetDecal%20Fade%20Size%20Multiplier))) 0))

(event Input|ActionEvents|InputActionFire
  (params (Key :type Key%20Structure :default "None"))
  (bind (_aimtransform_location _returnvalue) (|ConeRecoilWorkout_3))
  (bind (_aimtransform_location_2 _returnvalue_2) (|ConeRecoilWorkout))
  (bind (_aimtransform_location_3 _returnvalue_3) (|ConeRecoilWorkout_2))
  (bind _recoiltype (Variables|RecoilOptions|GetRecoilType))
  (bind _aimtransform (Variables|AimOffset|GetAimTransform))
  (bind _recoiltype_2 (Variables|RecoilOptions|GetRecoilType))
  (bind _aimtransform_2 (Variables|AimOffset|GetAimTransform))
  (bind _recoiltype_3 (Variables|RecoilOptions|GetRecoilType))
  (bind _aimtransform_3 (Variables|AimOffset|GetAimTransform))
  (bind _returnvalue_4 (Utilities|Select :Index _recoiltype :NewEnumerator0 _aimtransform_3 :NewEnumerator1 _aimtransform_3 :NewEnumerator2 (Math|Transform|MakeTransform _aimtransform_location _returnvalue "1,1,1")))
  (bind _returnvalue_5 (Utilities|Select :Index _recoiltype_2 :NewEnumerator0 _aimtransform :NewEnumerator1 _aimtransform :NewEnumerator2 (Math|Transform|MakeTransform _aimtransform_location_2 _returnvalue_2 "1,1,1")))
  (bind _returnvalue_6 (Utilities|Select :Index _recoiltype_3 :NewEnumerator0 _aimtransform_2 :NewEnumerator1 _aimtransform_2 :NewEnumerator2 (Math|Transform|MakeTransform _aimtransform_location_3 _returnvalue_3 "1,1,1")))
  ;[1 1 1] Trigger Press
  (:Pressed
    (Variables|Default|SetTriggerPressed true)
    (|FireRateAndSpamClickRegulation (Utilities|Select :Index (Variables|MyCharacter|GetSelectedWeapon) :Option%200 (Variables|FireRate|GetRifle%20Fire%20Rate) :Option%201 (Variables|FireRate|GetPistol%20Fire%20Rate) :Option%202 (Variables|FireRate|GetHiPowered%20Fire%20Rate) :Option%203 (Variables|FireRate|GetThrowGrenadeRate)) :!label _label
      (:FireProjectile
        (CallFunction|MuzzleSmokeOff)
        (CallFunction|AimOffsetTrigger)
        (switch int (Variables|MyCharacter|GetSelectedWeapon)
          (:0
            ;[1 1 1] Spawn Rifle projectile
            (if (Variables|Default|GetAiming)
              _
              (else
                (Animation|Montage|MontagePlay (Components|SkeletalMesh|GetAnimInstance (Variables|MyCharacter|GetMesh2P)) "/Game/BallisticsVFX/FirstPersonBPExamples/FirstPersonAssets/Animations/FirstPersonFire_Montage.FirstPersonFire_Montage" 1.0 "MontageLength" 0.0 true)))
            (Game|SpawnActorfromClass "/Game/BallisticsVFX/FXSpawnerBlueprints/Projectiles/CubitUniProjectile.CubitUniProjectile_C" (Math|Transform|MakeTransform (.location _returnvalue_5) (.rotation _returnvalue_5) "1,1,1") "AlwaysSpawn" 0 3e+04 true true false "NewEnumerator1" 0 "NewEnumerator0" 0) ; Spawn projectile
            (if (Variables|MyCharacter|GetGunAudioToggle)
              (Audio|SpawnSoundAttached "/Game/BallisticsVFX/SFX/Guns/Rifle_fire.Rifle_fire" (Variables|Default|GetProjectileSpawnPoint) "None" "0, 0, 0" "0, 0, 0" "KeepRelativeOffset" false 1.0 (Class|GameplayStatics|GetGlobalTimeDilation) 0.0 0 0))
            ;[1 1 1] Muzzle Flash
            (Effects|SpawnEmitterAttached "/Game/BallisticsVFX/Particles/Muzzle/MuzzleFlash/Muzzle_Flash_Med.Muzzle_Flash_Med" (Variables|Default|GetProjectileSpawnPoint) "None" (Transformation|GetSocketLocation (Variables|Default|GetProjectileSpawnPoint) "None") (Math|Rotator|CombineRotators (Pawn|GetControlRotation :!class /Script/Engine.Pawn) "0, 0, 0") "1.000000,1.000000,1.000000" "KeepWorldPosition")
            ;[1 1 1] Shell and Ejector Port Smoke
            (Effects|SpawnEmitteratLocation "/Game/BallisticsVFX/Particles/BulletCasings/Bullet_Casing_2.Bullet_Casing_2" (Transformation|GetSocketLocation (Variables|Default|GetEjectorPort) "None") (Math|Rotator|CombineRotators (Pawn|GetControlRotation :!class /Script/Engine.Pawn) "0,90.000000, 0"))
            (switch Utilities|FlowControl|Switch|SwitchonRecoilType (Variables|RecoilOptions|GetRecoilType)
              (:NewEnumerator1
                ;[1 1 1] Recoil Rifle Fire
                (bind _recoil_float (Timeline|Timeline_0 PlayFromStart)
                  (:Update
                    (Pawn|Input|AddControllerPitchInput (* (* (* _recoil_float (Variables|CameraRecoil|GetRifle_Recoil%20Amp)) (Math|Random|RandomFloatinRange 0.9 1.1)) (Variables|Default|GetBaseLookUpRate) (Utilities|Time|GetWorldDeltaSeconds)))
                    (Pawn|Input|AddControllerYawInput (* (* (* (* (* _recoil_float (Variables|CameraRecoil|GetRifle_Recoil%20Amp)) (Math|Random|RandomFloatinRange 0.9 1.1)) (Variables|CameraRecoil|GetRifle_sideways)) (Math|Random|RandomFloatinRange -1.0 1.0)) (Variables|Default|GetBaseTurnRate) (Utilities|Time|GetWorldDeltaSeconds))))))
              (:NewEnumerator2
                (CallFunction|ConeRecoil))))
          (:1
            ;[1 1 1] Spawn Pistol projectile
            (if (Variables|Default|GetAiming)
              _
              (else
                (Animation|Montage|MontagePlay (Components|SkeletalMesh|GetAnimInstance (Variables|MyCharacter|GetMesh2P)) "/Game/BallisticsVFX/FirstPersonBPExamples/FirstPersonAssets/Animations/FirstPersonFire_Montage.FirstPersonFire_Montage" 1.0 "MontageLength" 0.0 true)))
            (Game|SpawnActorfromClass "/Game/BallisticsVFX/FXSpawnerBlueprints/Projectiles/CubitUniProjectile.CubitUniProjectile_C" (Math|Transform|MakeTransform (.location _returnvalue_6) (.rotation _returnvalue_6) "1,1,1") "AlwaysSpawn" 0 1.5e+04 true true false "NewEnumerator1" 0 "NewEnumerator0" 0) ; Spawn projectile
            (if (Variables|MyCharacter|GetGunAudioToggle)
              (Audio|SpawnSoundAttached "/Game/BallisticsVFX/SFX/Guns/Pistol_fire.Pistol_fire" (Variables|Default|GetProjectileSpawnPoint) "None" "0, 0, 0" "0, 0, 0" "KeepRelativeOffset" false 1.0 (Class|GameplayStatics|GetGlobalTimeDilation) 0.0 0 0))
            ;[1 1 1] Muzzle Flash
            (Effects|SpawnEmitterAttached "/Game/BallisticsVFX/Particles/Muzzle/MuzzleFlash/Muzzle_Flash_Small.Muzzle_Flash_Small" (Variables|Default|GetProjectileSpawnPoint) "None" (Transformation|GetSocketLocation (Variables|Default|GetProjectileSpawnPoint) "None") (Math|Rotator|CombineRotators (Pawn|GetControlRotation :!class /Script/Engine.Pawn) "0, 0, 0") "1.000000,1.000000,1.000000" "KeepWorldPosition")
            ;[1 1 1] Shell and Ejector Port Smoke
            (Effects|SpawnEmitteratLocation "/Game/BallisticsVFX/Particles/BulletCasings/Bullet_Casing_2.Bullet_Casing_2" (Transformation|GetSocketLocation (Variables|Default|GetEjectorPort) "None") (Math|Rotator|CombineRotators (Pawn|GetControlRotation :!class /Script/Engine.Pawn) "0,90.000000, 0"))
            (switch Utilities|FlowControl|Switch|SwitchonRecoilType (Variables|RecoilOptions|GetRecoilType)
              (:NewEnumerator1
                ;[1 1 1] Recoil Pistol Fire
                (bind _recoil_float_2 (Timeline|Timeline_1 PlayFromStart)
                  (:Update
                    (Pawn|Input|AddControllerPitchInput (* (* (* _recoil_float_2 (Variables|CameraRecoil|GetPistol_Recoil%20Amp)) (Math|Random|RandomFloatinRange 0.9 1.1)) (Variables|Default|GetBaseLookUpRate) (Utilities|Time|GetWorldDeltaSeconds)))
                    (Pawn|Input|AddControllerYawInput (* (* (* (* (* _recoil_float_2 (Variables|CameraRecoil|GetPistol_Recoil%20Amp)) (Math|Random|RandomFloatinRange 0.9 1.1)) (Variables|CameraRecoil|GetPistol_sideways)) (Math|Random|RandomFloatinRange -1.0 1.0)) (Variables|Default|GetBaseTurnRate) (Utilities|Time|GetWorldDeltaSeconds))))))
              (:NewEnumerator2
                (CallFunction|ConeRecoil))))
          (:2
            ;[1 1 1] Spawn HP Rifle projectile
            (if (Variables|Default|GetAiming)
              _
              (else
                (Animation|Montage|MontagePlay (Components|SkeletalMesh|GetAnimInstance (Variables|MyCharacter|GetMesh2P)) "/Game/BallisticsVFX/FirstPersonBPExamples/FirstPersonAssets/Animations/FirstPersonFire_Montage.FirstPersonFire_Montage" 1.0 "MontageLength" 0.0 true)))
            (Game|SpawnActorfromClass "/Game/BallisticsVFX/FXSpawnerBlueprints/Projectiles/CubitUniProjectile.CubitUniProjectile_C" (Math|Transform|MakeTransform (.location _returnvalue_4) (.rotation _returnvalue_4) "1,1,1") "AlwaysSpawn" 0 4e+04 true true false "NewEnumerator2" 0 "NewEnumerator0" 0) ; Spawn projectile
            (if (Variables|MyCharacter|GetGunAudioToggle)
              (Audio|SpawnSoundAttached "/Game/BallisticsVFX/SFX/Guns/HiPowered.HiPowered" (Variables|Default|GetProjectileSpawnPoint) "None" "0, 0, 0" "0, 0, 0" "KeepRelativeOffset" false 1.0 (Class|GameplayStatics|GetGlobalTimeDilation) 0.0 0 0))
            ;[1 1 1] Muzzle Flash
            (Effects|SpawnEmitterAttached "/Game/BallisticsVFX/Particles/Muzzle/MuzzleFlash/Muzzle_Flash_Med.Muzzle_Flash_Med" (Variables|Default|GetProjectileSpawnPoint) "None" (Transformation|GetSocketLocation (Variables|Default|GetProjectileSpawnPoint) "None") (Math|Rotator|CombineRotators (Pawn|GetControlRotation :!class /Script/Engine.Pawn) "0, 0, 0") "1.000000,1.000000,1.000000" "KeepWorldPosition")
            ;[1 1 1] Shell and Ejector Port Smoke
            (Effects|SpawnEmitteratLocation "/Game/BallisticsVFX/Particles/BulletCasings/Bullet_Casing_2.Bullet_Casing_2" (Transformation|GetSocketLocation (Variables|Default|GetEjectorPort) "None") (Math|Rotator|CombineRotators (Pawn|GetControlRotation :!class /Script/Engine.Pawn) "0,90.000000, 0"))
            (switch Utilities|FlowControl|Switch|SwitchonRecoilType (Variables|RecoilOptions|GetRecoilType)
              (:NewEnumerator1
                ;[1 1 1] Recoil Hi Powered Fire
                (bind _recoil_float_3 (Timeline|Timeline_5 PlayFromStart)
                  (:Update
                    (Pawn|Input|AddControllerPitchInput (* (* (* _recoil_float_3 (Variables|CameraRecoil|GetHP_Recoil%20Amp)) (Math|Random|RandomFloatinRange 0.9 1.1)) (Variables|Default|GetBaseLookUpRate) (Utilities|Time|GetWorldDeltaSeconds)))
                    (Pawn|Input|AddControllerYawInput (* (* (* (* (* _recoil_float_3 (Variables|CameraRecoil|GetHP_Recoil%20Amp)) (Math|Random|RandomFloatinRange 0.9 1.1)) (Variables|CameraRecoil|GetHP_sideways)) (Math|Random|RandomFloatinRange -0.5 0.5)) (Variables|Default|GetBaseTurnRate) (Utilities|Time|GetWorldDeltaSeconds))))))
              (:NewEnumerator2
                (CallFunction|ConeRecoil))))
          (:3
            ;[1 1 1] Grenade Thrown
            (Game|SpawnActorfromClass "/Game/BallisticsVFX/FXSpawnerBlueprints/Projectiles/Grenade_Thrown.Grenade_Thrown_C" (Math|Transform|MakeTransform (Transformation|GetSocketLocation (Variables|Default|GetGrenadeSpawnPoint) "None") (Pawn|GetControlRotation :!class /Script/Engine.Pawn)) "AdjustIfPossibleButDontSpawnIfColliding" 0 true 25 0 :!pinned true) ; Spawn projectile
            (Audio|SpawnSoundAttached "/Game/BallisticsVFX/SFX/Whoosh/Whoosh_1_Cue.Whoosh_1_Cue" (Variables|Default|GetGrenadeSpawnPoint) "None" "0, 0, 0" "0, 0, 0" "KeepRelativeOffset" false 1.0 (Class|GameplayStatics|GetGlobalTimeDilation) 0.0 0 0))))))
  (:Released
    (Variables|Default|SetTriggerPressed false)
    (CallFunction|TriggerOFF)
    (goto _label TriggerOFF)))

(event Input|KeyboardEvents|F
  (params (Key :type Key%20Structure :default "None"))
  (bind _firstpersoncamera (Variables|MyCharacter|GetFirstPersonCamera))
  (bind _returnvalue (Transformation|GetWorldLocation _firstpersoncamera))
  ;[1 1 1] Fire raytrace, good for testing!!!
  (:Pressed
    (bind (_outhit _returnvalue_2) (Collision|LineTraceByChannel _returnvalue (+ _returnvalue (* (Math|Vector|GetForwardVector (Transformation|GetWorldRotation _firstpersoncamera)) 8e+03)) "TraceTypeQuery1" false 0 "ForDuration" true "(R=1.000000,G=0.000000,B=0.000000,A=1.000000)" "(R=0.000000,G=1.000000,B=0.000000,A=1.000000)" 1.0))
    (if _returnvalue_2
      (Development|PrintString (Utilities|GetDisplayName (.HitComponent (Collision|BreakHitResult _outhit))))
      (if (Variables|Default|GetObjectPickedUp)
        (Class|BPIInteraction|BPIInteraction(Message) (.HitActor (Collision|BreakHitResult _outhit)) self (.HitComponent (Collision|BreakHitResult _outhit)) (Variables|Default|GetPickup))
        (else
          (Class|BPIInteraction|BPIInteraction(Message) (.HitActor (Collision|BreakHitResult _outhit)) self (.HitComponent (Collision|BreakHitResult _outhit))))))))

(event Input|MouseEvents|RightMouseButton
  (params (Key :type Key%20Structure :default "None"))
  ;[1 1 1] Grenade Launcher
  (:Pressed
    (Game|SpawnActorfromClass "/Game/BallisticsVFX/FXSpawnerBlueprints/Projectiles/Grenade_launched.Grenade_launched_C" (Math|Transform|MakeTransform (Transformation|GetSocketLocation (Variables|Default|GetGrenadeSpawnPoint) "None") (Pawn|GetControlRotation :!class /Script/Engine.Pawn)) "AdjustIfPossibleButDontSpawnIfColliding" 0 true 0 :!pinned true) ; Spawn projectile
    (Audio|SpawnSoundAttached "/Game/BallisticsVFX/SFX/GrenLauncher/GrenadeLauncher_cue.GrenadeLauncher_cue" (Variables|Default|GetProjectileSpawnPoint) "None" "0, 0, 0" "0, 0, 0" "KeepRelativeOffset" false 1.0 (Class|GameplayStatics|GetGlobalTimeDilation) 0.0 0 0)
    (switch Utilities|FlowControl|Switch|SwitchonRecoilType (Variables|RecoilOptions|GetRecoilType)
      (:NewEnumerator1
        ;[1 1 1] Recoil Grenade Fire
        (bind _recoil_float (Timeline|Timeline_6 PlayFromStart)
          (:Update
            (Pawn|Input|AddControllerPitchInput (* (* (* _recoil_float (Variables|CameraRecoil|GetGrenadeLauncher_Recoil)) (Math|Random|RandomFloatinRange 0.9 1.1)) (Variables|Default|GetBaseLookUpRate) (Utilities|Time|GetWorldDeltaSeconds)))
            (Pawn|Input|AddControllerYawInput (* (* (* (* (* _recoil_float (Variables|CameraRecoil|GetGrenadeLauncher_Recoil)) (Math|Random|RandomFloatinRange 0.9 1.1)) (Variables|CameraRecoil|GetGrenade_sideways)) (Math|Random|RandomFloatinRange -1.0 1.0)) (Variables|Default|GetBaseTurnRate) (Utilities|Time|GetWorldDeltaSeconds))))))
      (:NewEnumerator2
        (CallFunction|ConeRecoil)))))

(fn ConstructionScript
  (Class|SceneComponent|Attachto (Variables|Default|GetFP_Gun) (Variables|MyCharacter|GetMesh2P) "GripPoint" "SnapToTargetIncludingScale" true))