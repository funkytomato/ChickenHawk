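; Master ballistics gun that fires rifle, pistol and high-powered projectiles or throws grenades, with a separate event for launched grenades.
; Fire input runs through a gate and retriggerable-delay macro that repeats shots while held and blocks spam-clicking, then switches on SelectedWeapon to spawn projectiles, sounds and effects.
; Muzzle smoke starts on trigger release to avoid stacking during rapid fire, and Tick cuts it during fast movement or while firing.
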(event Custom|LaunchGrenade
  ;[1 1 1] Grenade Launcher
  (Game|SpawnActorfromClass "/Game/BallisticsVFX/FXSpawnerBlueprints/Projectiles/Grenade_launched.Grenade_launched_C" (Math|Transform|MakeTransform (Transformation|GetSocketLocation (Variables|Gun|GetGrenadeSpawnPoint) "None") (Pawn|GetControlRotation (Variables|Default|GetGunOwner) :!class /Script/Engine.Pawn)) "AdjustIfPossibleButDontSpawnIfColliding" 0 true 0 :!pinned true) ; Spawn projectile
  (Audio|SpawnSoundAttached "/Game/BallisticsVFX/SFX/GrenLauncher/GrenadeLauncher_cue.GrenadeLauncher_cue" 0 "None" "0, 0, 0" "0, 0, 0" "KeepRelativeOffset" false 1.0 (Class|GameplayStatics|GetGlobalTimeDilation) 0.0 0 0))

(event Custom|TriggerOFF
  ;[0.2075 0.4327 1] Activate Muzzle Smoke FX once trigger is lifted (we don't want to spawn too many smoke FX during rapid fire)
  (Components|Activation|Activate (Variables|Gun|GetMuzzle%20Smoke%20Light) false))

(event Custom|TriggerON
  ;[0.2075 0.4327 1] Activate Muzzle Smoke FX once trigger is lifted (we don't want to spawn too many smoke FX during rapid fire)
  (CallFunction|MuzzleSmokeOff))

(event Custom|MuzzleSmokeOff
  ;[0.2075 0.4327 1] MUZZLE SMOKE OFF
  (Components|Activation|Deactivate (Variables|Gun|GetMuzzle%20Smoke%20Light)))

(event EventTick
  (params (DeltaSeconds :type Float%20%28single-precision%29))
  ;[1 1 1] Movement Check Each Tick
  (if (>= (Math|Vector|VectorLength (Transformation|GetVelocity (Pawn|GetMovementBaseActor (Variables|Default|GetGunOwner)))) 8e+02)
    (Variables|Default|SetCharacterMoving true)
    ;[0.2075 0.4327 1] Deactivate Muzzle Smoke On Movement Threshold
    (if (Components|Activation|IsActive (Variables|Gun|GetMuzzle_Smoke_light)) :!label _label
      (CallFunction|MuzzleSmokeOff))
    (else
      (Variables|Default|SetCharacterMoving false)
      (if (Variables|Default|GetTriggerPressed)
        (goto _label)))))

(event Input|ActionEvents|InputActionFire
  (params (Key :type Key%20Structure :default "None"))
  (bind (_aimtransform_location _returnvalue) (|ConeRecoilWorkout_3_2))
  (bind (_aimtransform_location_2 _returnvalue_2) (|ConeRecoilWorkout_2))
  (bind (_aimtransform_location_3 _returnvalue_3) (|ConeRecoilWorkout_2_2))
  (bind _recoiltype (Variables|Default|GetRecoilType))
  (bind _recoiltype_2 (Variables|Default|GetRecoilType))
  (bind _recoiltype_3 (Variables|Default|GetRecoilType))
  (bind _returnvalue_4 (Utilities|Select :Index _recoiltype :NewEnumerator0 "" :NewEnumerator1 "" :NewEnumerator2 (Math|Transform|MakeTransform _aimtransform_location _returnvalue "1,1,1")))
  (bind _returnvalue_5 (Utilities|Select :Index _recoiltype_2 :NewEnumerator0 "" :NewEnumerator1 "" :NewEnumerator2 (Math|Transform|MakeTransform _aimtransform_location_2 _returnvalue_2 "1,1,1")))
  (bind _returnvalue_6 (Utilities|Select :Index _recoiltype_3 :NewEnumerator0 "" :NewEnumerator1 "" :NewEnumerator2 (Math|Transform|MakeTransform _aimtransform_location_3 _returnvalue_3 "1,1,1")))
  ;[1 1 1] Trigger Press
  (:Pressed
    (Variables|Default|SetTriggerPressed true)
    (|FireRateAndSpamClickRegulation_2 (Utilities|Select :Index (Variables|Default|GetSelectedWeapon) :Option%200 (Variables|FireRate|GetRifle%20Fire%20Rate) :Option%201 (Variables|FireRate|GetPistol%20Fire%20Rate) :Option%202 (Variables|FireRate|GetHiPowered%20Fire%20Rate) :Option%203 (Variables|FireRate|GetThrowGrenadeRate)) :!label _label
      (:FireProjectile
        (CallFunction|MuzzleSmokeOff)
        (switch int (Variables|Default|GetSelectedWeapon)
          (:0
            ;[1 1 1] Spawn Rifle projectile
            (Game|SpawnActorfromClass "/Game/BallisticsVFX/FXSpawnerBlueprints/Projectiles/CubitUniProjectile.CubitUniProjectile_C" (Math|Transform|MakeTransform (.location _returnvalue_5) (.rotation _returnvalue_5) "1,1,1") "AlwaysSpawn" 0 3e+04 true true false "NewEnumerator1" 0 "NewEnumerator0" 0) ; Spawn projectile
            (if (Variables|Default|GetGunAudioToggle)
              (Audio|SpawnSoundAttached "/Game/BallisticsVFX/SFX/Guns/Rifle_fire.Rifle_fire" (Variables|Gun|GetProjectileSpawnPoint) "None" "0, 0, 0" "0, 0, 0" "KeepRelativeOffset" false 1.0 (Class|GameplayStatics|GetGlobalTimeDilation) 0.0 0 0))
            ;[1 1 1] Muzzle Flash
            (Effects|SpawnEmitterAttached "/Game/BallisticsVFX/Particles/Muzzle/MuzzleFlash/Muzzle_Flash_Med.Muzzle_Flash_Med" (Variables|Gun|GetProjectileSpawnPoint) "None" (Transformation|GetSocketLocation (Variables|Gun|GetProjectileSpawnPoint) "None") (Math|Rotator|CombineRotators (Pawn|GetControlRotation (Variables|Default|GetGunOwner) :!class /Script/Engine.Pawn) "0, 0, 0") "1.000000,1.000000,1.000000" "KeepWorldPosition")
            ;[1 1 1] Shell and Ejector Port Smoke
            (Effects|SpawnEmitteratLocation "/Game/BallisticsVFX/Particles/BulletCasings/Bullet_Casing_2.Bullet_Casing_2" (Transformation|GetSocketLocation (Variables|Gun|GetEjectorPort) "None") (Math|Rotator|CombineRotators (Pawn|GetControlRotation (Variables|Default|GetGunOwner) :!class /Script/Engine.Pawn) "0,90.000000, 0")))
          (:1
            ;[1 1 1] Spawn Pistol projectile
            (Game|SpawnActorfromClass "/Game/BallisticsVFX/FXSpawnerBlueprints/Projectiles/CubitUniProjectile.CubitUniProjectile_C" (Math|Transform|MakeTransform (.location _returnvalue_6) (.rotation _returnvalue_6) "1,1,1") "AlwaysSpawn" 0 1.5e+04 true true false "NewEnumerator1" 0 "NewEnumerator0" 0) ; Spawn projectile
            (if (Variables|Default|GetGunAudioToggle)
              (Audio|SpawnSoundAttached "/Game/BallisticsVFX/SFX/Guns/Pistol_fire.Pistol_fire" 0 "None" "0, 0, 0" "0, 0, 0" "KeepRelativeOffset" false 1.0 (Class|GameplayStatics|GetGlobalTimeDilation) 0.0 0 0))
            ;[1 1 1] Muzzle Flash
            (Effects|SpawnEmitterAttached "/Game/BallisticsVFX/Particles/Muzzle/MuzzleFlash/Muzzle_Flash_Small.Muzzle_Flash_Small" (Variables|Gun|GetProjectileSpawnPoint) "None" (Transformation|GetSocketLocation (Variables|Gun|GetProjectileSpawnPoint) "None") (Math|Rotator|CombineRotators (Pawn|GetControlRotation (Variables|Default|GetGunOwner) :!class /Script/Engine.Pawn) "0, 0, 0") "1.000000,1.000000,1.000000" "KeepWorldPosition")
            ;[1 1 1] Shell and Ejector Port Smoke
            (Effects|SpawnEmitteratLocation "/Game/BallisticsVFX/Particles/BulletCasings/Bullet_Casing_2.Bullet_Casing_2" (Transformation|GetSocketLocation (Variables|Gun|GetEjectorPort) "None") (Math|Rotator|CombineRotators (Pawn|GetControlRotation (Variables|Default|GetGunOwner) :!class /Script/Engine.Pawn) "0,90.000000, 0")))
          (:2
            ;[1 1 1] Spawn HP Rifle projectile
            (Game|SpawnActorfromClass "/Game/BallisticsVFX/FXSpawnerBlueprints/Projectiles/CubitUniProjectile.CubitUniProjectile_C" (Math|Transform|MakeTransform (.location _returnvalue_4) (.rotation _returnvalue_4) "1,1,1") "AlwaysSpawn" 0 4e+04 true true false "NewEnumerator2" 0 "NewEnumerator0" 0) ; Spawn projectile
            (if (Variables|Default|GetGunAudioToggle)
              (Audio|SpawnSoundAttached "/Game/BallisticsVFX/SFX/Guns/HiPowered.HiPowered" 0 "None" "0, 0, 0" "0, 0, 0" "KeepRelativeOffset" false 1.0 (Class|GameplayStatics|GetGlobalTimeDilation) 0.0 0 0))
            ;[1 1 1] Muzzle Flash
            (Effects|SpawnEmitterAttached "/Game/BallisticsVFX/Particles/Muzzle/MuzzleFlash/Muzzle_Flash_Med.Muzzle_Flash_Med" (Variables|Gun|GetProjectileSpawnPoint) "None" (Transformation|GetSocketLocation (Variables|Gun|GetProjectileSpawnPoint) "None") (Math|Rotator|CombineRotators (Pawn|GetControlRotation (Variables|Default|GetGunOwner) :!class /Script/Engine.Pawn) "0, 0, 0") "1.000000,1.000000,1.000000" "KeepWorldPosition")
            ;[1 1 1] Shell and Ejector Port Smoke
            (Effects|SpawnEmitteratLocation "/Game/BallisticsVFX/Particles/BulletCasings/Bullet_Casing_2.Bullet_Casing_2" (Transformation|GetSocketLocation (Variables|Gun|GetEjectorPort) "None") (Math|Rotator|CombineRotators (Pawn|GetControlRotation (Variables|Default|GetGunOwner) :!class /Script/Engine.Pawn) "0,90.000000, 0")))
          (:3
            ;[1 1 1] Grenade Thrown
            (Game|SpawnActorfromClass "/Game/BallisticsVFX/FXSpawnerBlueprints/Projectiles/Grenade_Thrown.Grenade_Thrown_C" (Math|Transform|MakeTransform (Transformation|GetSocketLocation (Variables|Gun|GetGrenadeSpawnPoint) "None") (Pawn|GetControlRotation (Variables|Default|GetGunOwner) :!class /Script/Engine.Pawn)) "AdjustIfPossibleButDontSpawnIfColliding" 0 true 25 0 :!pinned true) ; Spawn projectile
            (Audio|SpawnSoundAttached "/Game/BallisticsVFX/SFX/Whoosh/Whoosh_1_Cue.Whoosh_1_Cue" (Variables|Gun|GetGrenadeSpawnPoint) "None" "0, 0, 0" "0, 0, 0" "KeepRelativeOffset" false 1.0 (Class|GameplayStatics|GetGlobalTimeDilation) 0.0 0 0))))))
  (:Released
    (Variables|Default|SetTriggerPressed false)
    (CallFunction|TriggerOFF)
    (goto _label TriggerOFF)))

(event Input|KeyboardEvents|F
  (params (Key :type Key%20Structure :default "None"))
  ;[1 1 1] Fire raytrace, good for testing!!!
)

(fn ConstructionScript)