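; MGGun_BP is a stationary-prop machine gun that fires automatically on a looping one-second timer started at BeginPlay.
; Each shot plays sound and muzzle flash and spawns bullet and casing actors from the mesh's Muzzle and EjectionPort sockets.
; A sphere overlap tracks helicopter characters in a Targets array, but this graph never uses that list to aim or gate firing.
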(event OnComponentBeginOverlap(SphereOfInfluence)
  (params (OverlappedComponent :type Primitive%20Component%20Object%20Reference) (OtherActor :type Actor%20Object%20Reference) (OtherComp :type Primitive%20Component%20Object%20Reference) (OtherBodyIndex :type Integer) (bFromSweep :type Boolean) (SweepResult :type Hit%20Result%20Structure%20%28by%20ref%29))
  (Utilities|FlowControl|Sequence
    (:then_0
      (bind _ashelicopter_character_with_fixed_joystick (Utilities|Casting|CastToHelicopterCharacterWithFixedJoystick OtherActor))
      (Utilities|Array|Add (Variables|GunTargeting|GetTargets) _ashelicopter_character_with_fixed_joystick))))

(event OnComponentEndOverlap(SphereOfInfluence)
  (params (OverlappedComponent :type Primitive%20Component%20Object%20Reference) (OtherActor :type Actor%20Object%20Reference) (OtherComp :type Primitive%20Component%20Object%20Reference) (OtherBodyIndex :type Integer))
  (Utilities|FlowControl|Sequence
    (:then_0
      (bind _ashelicopter_character_with_fixed_joystick (Utilities|Casting|CastToHelicopterCharacterWithFixedJoystick OtherActor))
      (Utilities|Array|RemoveItem (Variables|GunTargeting|GetTargets) _ashelicopter_character_with_fixed_joystick))))

(event Custom|FireGun
  (bind _sm_prop_mg_stand_01 (Variables|Gun|GetSM_Prop_Mg_stand_01))
  (bind _returnvalue (Transformation|GetSocketLocation _sm_prop_mg_stand_01 "Muzzle"))
  (Audio|PlaySoundatLocation "/Game/MyContent/Assets/Audio/Effects/Gun_M16_1Shot_01_Cue.Gun_M16_1Shot_01_Cue" _returnvalue "0, 0, 0" 1.0 1.0 0.0 0 0 0)
  (Effects|SpawnEmitteratLocation "/Game/PolygonHeist/ParticleFX/FX_Gunshot.FX_Gunshot" _returnvalue (Transformation|GetSocketRotation _sm_prop_mg_stand_01 "Muzzle"))
  (Game|SpawnActorfromClass "/Game/MyContent/Projectiles/Blueprints/MG_Casing_BP.MG_Casing_BP_C" (Transformation|GetSocketTransform _sm_prop_mg_stand_01 "EjectionPort" "RTS_World") "AlwaysSpawn" 0 0)
  (Game|SpawnActorfromClass "/Game/MyContent/Projectiles/Blueprints/MG_Bullet_BP.MG_Bullet_BP_C" (Transformation|GetSocketTransform _sm_prop_mg_stand_01 "Muzzle" "RTS_World") "AlwaysSpawn" 0 0))

(event EventBeginPlay
  (Utilities|Time|SetTimerbyFunctionName 0 "FireGun" 1.0 true))

(fn ConstructionScript)