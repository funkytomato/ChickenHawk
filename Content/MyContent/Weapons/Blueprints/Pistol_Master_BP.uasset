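; Master pistol Blueprint that provides the cosmetic effects for firing and reloading a handgun.
; FirePistol plays a sound and emitter at the Muzzle socket, spawns an actor at the Ejection Port socket and plays a one-shot mesh animation.
; ReloadMagazine spawns an actor at the Magazine socket.
; The graph contains no projectile, trace, damage or ammo logic.
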(event Custom|Fire%20Pistol
  (bind _skeletalmesh (Variables|Default|GetSkeletalMesh))
  (bind _returnvalue (Transformation|GetSocketLocation _skeletalmesh "Muzzle"))
  (Audio|PlaySoundatLocation 0 _returnvalue "0, 0, 0" 1.0 1.0 0.0 0 0 0)
  (Effects|SpawnEmitteratLocation 0 _returnvalue (Transformation|GetSocketRotation _skeletalmesh "Muzzle"))
  (Game|SpawnActorfromClass 0 (Transformation|GetSocketTransform _skeletalmesh "Ejection Port" "RTS_World") "Undefined" 0 0)
  (Components|Animation|PlayAnimation (Variables|Default|GetSkeletalMesh) 0 false))

(event Custom|Reload%20Magazine
  (Game|SpawnActorfromClass 0 (Transformation|GetSocketTransform (Variables|Default|GetSkeletalMesh) "Magazine" "RTS_World") "Undefined" 0 0))

(fn ConstructionScript)