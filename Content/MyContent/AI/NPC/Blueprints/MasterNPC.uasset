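; Base NPC character that wanders between random reachable nav points and carries an M5 rifle it can draw, holster, fire and reload.
; Gun actions are bound to debug-style key inputs and pass through authority checks into Client events, as does death on zero health, which plays an animation and unpossesses.
; A sphere overlap collects attackable targets for selection, while combat-state events only print and patrol-point and respawn logic is disconnected.
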(event OnComponentBeginOverlap(SphereOfInfluence)
  (params (OverlappedComponent :type Primitive%20Component%20Object%20Reference) (OtherActor :type Actor%20Object%20Reference) (OtherComp :type Primitive%20Component%20Object%20Reference) (OtherBodyIndex :type Integer) (bFromSweep :type Boolean) (SweepResult :type Hit%20Result%20Structure%20%28by%20ref%29))
  ;[1 1 1] Attackable Target detected, add to list of Targets
  (bind _asattackable_master_bp (Utilities|Casting|CastToAttackableMaster_BP OtherActor))
  (if (Variables|/Game/MyContent/Buildings/Blueprints/AttackableMaster_BP.AttackableMaster_BP_C|GetAttackable _asattackable_master_bp)
    (Utilities|Array|AddUnique (Variables|Default|GetTargets) 0)))

(event Custom|Client%20Holster%20Gun
  ;[1 1 1] Gun Functionality
  (Rendering|SetVisibility (Variables|Default|GetHolsteredGun) true false)
  (Actor|DestroyActor (Variables|Gun|GetGunInHand))
  (Variables|Gun|SetGunEquipped false)
  (Variables|Gun|SetCanShoot false))

(event Custom|Holster%20Gun
  ;[1 1 1] Gun Functionality
  (Networking|SwitchHasAuthority
    (:Authority
      (CallFunction|ClientHolsterGun))))

(event Custom|Death
  ;[1 1 1] OnDeath
  (Networking|SwitchHasAuthority
    (:Authority
      (CallFunction|ClientDeath))))

(event Custom|Client%20Death
  ;[1 1 1] OnDeath
  (Pawn|Components|CharacterMovement|SetMovementMode (Variables|Character|GetCharacterMovement) "MOVE_None" 0)
  (Components|Animation|PlayAnimation (Variables|Character|GetMesh) "/Game/MyContent/Characters/Animations/Synty/Commando/Death_1.Death_1" false)
  ;;[1 1 1] Stop and disable the AIController
  (Actor|Tick|SetActorTickEnabled false)
  (Pawn|UnPossess (Pawn|GetController))
  (Variables|Character|SetIsDead? true))

(event Custom|Start%20Reloading%20Gun
  ;[1 1 1] Reload Gun
  (Networking|SwitchHasAuthority
    (:Authority
      (CallFunction|ClientStartReloadGun))))

(event Custom|Configure%20AI%20Controller
  ;[1 1 1] Base Logic for Movement AI
  (bind _movementresult (AI|AIMoveTo self (.RandomLocation (AI|Navigation|GetRandomReachablePointinRadius (Transformation|GetActorLocation) 1e+03 0 0)) 0 1e+01 false)
    (:OnSuccess
      (Utilities|FlowControl|Delay 1.0)
      (if (not (Utilities|Enum|Equal(Enum) _movementresult "Invalid"))
        (CallFunction|GoPointAgain)
        (else
          (Development|PrintString "Failed AI movement"))))))

(event Custom|Attach%20Gun
  ;[1 1 1] Spawn and Attach Gun to Character
  (CallFunction|SpawnM5))

(event Custom|GetNewTargetFromListOfTargets
  ;[1 1 1] Get a Target from the TargetList and set the CurrentTarget
  (Utilities|IsValid (Variables|Default|GetCurrentTarget)
    (:Is%20Valid
      (bind _returnvalue (Utilities|Array|RemoveItem (Variables|Default|GetTargets) 0))
      (if _returnvalue
        (if (Utilities|Array|IsValidIndex (Variables|Default|GetTargets)) :!label _label
          (Variables|Default|SetCurrentTarget (Utilities|Array|Get(acopy) (Variables|Default|GetTargets)))
          (else
            (Development|PrintString "No targets")))
        (else
          (Development|PrintString "Failed to find target in Targets array"))))
    (:Is%20Not%20Valid
      (goto _label))))

(event Custom|Client%20Draw%20Gun
  ;[1 1 1] Gun Functionality
  (Rendering|SetVisibility (Variables|Default|GetHolsteredGun) false false)
  (bind _returnvalue (Game|SpawnActorfromClass "/Game/MyContent/Weapons/Blueprints/M5Gun_BP.M5Gun_BP_C" (Transformation|GetSocketTransform (Variables|Character|GetMesh) (Variables|Gun|GetRightHand) "RTS_World") "Undefined" 0 0))
  (Variables|Gun|SetGunInHand _returnvalue)
  (Transformation|AttachComponentToComponent (Variables|Character|GetMesh) (Variables|Gun|GetRightHand) "SnapToTarget" "SnapToTarget" "SnapToTarget" true)
  (Variables|Gun|SetGunEquipped true)
  (Variables|Gun|SetCanShoot true)
  (Variables|Gun|SetCanReload true))

(event Custom|Draw%20Gun
  ;[1 1 1] Gun Functionality
  (Networking|SwitchHasAuthority
    (:Authority
      (CallFunction|ClientDrawGun))))

(event Custom|Client%20Fire%20Gun
  ;[1 1 1] Fire Rifle
  (bind _asmaster_ballistics_gun_bp (Utilities|Casting|CastToMasterBallisticsGun_BP (Variables|Gun|GetGunInHand)))
  (Default|FireGun _asmaster_ballistics_gun_bp))

(event Custom|Fire%20Gun
  ;[1 1 1] Fire Rifle
  (Networking|SwitchHasAuthority
    (:Authority
      (CallFunction|ClientFireGun))))

(event Custom|Client%20Start%20Reload%20Gun
  ;[1 1 1] Reload Gun
  (if (Variables|Gun|GetCanReload)
    (Variables|Gun|SetReloadGun true)
    (Variables|Gun|SetCanShoot false)
    (bind _asm5gun_bp (Utilities|Casting|CastToM5Gun_BP (Variables|Gun|GetGunInHand)))
    (Default|ReloadMagazine _asm5gun_bp)
    (Utilities|FlowControl|Delay 1.667)
    (Variables|Gun|SetCanReload true)
    (Variables|Gun|SetCanShoot true)))

(event Custom|Client%20Stop%20Reload%20Gun
  ;[1 1 1] Reload Gun
  (Variables|Gun|SetReloadGun false))

(event Custom|GoPointAgain
  ;[1 1 1] Base Logic for Movement AI
  (bind _movementresult (AI|AIMoveTo self (.RandomLocation (AI|Navigation|GetRandomReachablePointinRadius (Transformation|GetActorLocation) 1e+03 0 0)) 0 1e+01 false)
    (:OnSuccess
      (Utilities|FlowControl|Delay 1.0)
      (if (not (Utilities|Enum|Equal(Enum) _movementresult "Invalid"))
        (CallFunction|GoPointAgain)
        (else
          (Development|PrintString "Failed AI movement"))))))

(event Custom|Stop%20Reloading%20Gun
  ;[1 1 1] Reload Gun
  (Networking|SwitchHasAuthority
    (:Authority
      (CallFunction|ClientStopReloadGun))))

(event Game|Damage|EventAnyDamage
  (params (Damage :type Float%20%28single-precision%29) (DamageType :type Damage%20Type%20Object%20Reference) (InstigatedBy :type Controller%20Object%20Reference) (DamageCauser :type Actor%20Object%20Reference))
  ;[1 1 1] Apply Damage to Player
  (bind _output_get (Variables|Character|SetHealth (- (Variables|Character|GetHealth) Damage)))
  (Variables|Character|SetIsHit true)
  (if (<= _output_get 0.0)
    (Variables|Character|SetHealth 0.0)
    (CallFunction|Death)
    (else
      (Utilities|FlowControl|Delay 0.5)
      (Variables|Character|SetIsHit false))))

(event EventBeginPlay
  ;[1 1 1] Beginplay - Spawn Gun to Rifle Holstered Position on Character
  (CallFunction|ConfigureAIController))

(event EventAttacking
  (params (AttackableTarget :type Actor%20Object%20Reference) (AttackableTargetType :type AttackableTarget%20Enum :default "NewEnumerator0"))
  (Development|PrintString "Attacking"))

(event EventDefending
  (params (LocationToDefend :type Vector :default "0, 0, 0"))
  (Development|PrintString "Defending"))

(event EventStandyby
  (Development|PrintString "StandyBy"))

(event EventRetreating
  (Development|PrintString "Retreating"))

(event EventCover
  (Development|PrintString "Cover"))

(event EventOntheMove
  (params (Destination :type Vector :default "0, 0, 0"))
  (Development|PrintString "OnTheMove"))

(event Input|KeyboardEvents|2
  (params (Key :type Key%20Structure :default "None"))
  ;[1 1 1] Gun Functionality
  (:Pressed
    (Utilities|FlowControl|FlipFlop
      (:A
        (CallFunction|DrawGun))
      (:B
        (CallFunction|HolsterGun)))))

(event Input|MouseEvents|LeftMouseButton
  (params (Key :type Key%20Structure :default "None"))
  ;[1 1 1] Fire Rifle
  (:Pressed
    (if (Variables|Gun|GetGunEquipped)
      (if (Variables|Gun|GetCanShoot)
        (CallFunction|FireGun)))))

(event Input|KeyboardEvents|R
  (params (Key :type Key%20Structure :default "None"))
  ;[1 1 1] Reload Gun
  (:Pressed
    (CallFunction|StartReloadingGun))
  (:Released
    (CallFunction|StopReloadingGun)))

(event Input|KeyboardEvents|F
  (params (Key :type Key%20Structure :default "None"))
  ;[1 1 1] Turn on Flashlight
)

(fn ConstructionScript)

(fn SpawnM5
  (bind _returnvalue (Game|SpawnActorfromClass "/Game/MyContent/Weapons/Blueprints/M5Gun_BP.M5Gun_BP_C" (Transformation|GetSocketTransform (Variables|Character|GetMesh) (Utilities|Name|MakeLiteralName "RifleHolsteredSocket") "RTS_World") "Undefined" 0 self))
  (Transformation|AttachComponentToComponent _returnvalue (Variables|Character|GetMesh) (Utilities|Name|MakeLiteralName "RifleHolsteredSocket") "SnapToTarget" "SnapToTarget" "SnapToTarget" true))