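; AI controller for the master NPC that runs its behavior tree and tracks the player as the enemy.
; On begin play it starts MasterNPC_BT and seeds the blackboard with pawn and player.
; Perception updates feed CompleteSenses, which treats stimulus index 0 as player visibility, records the player's location with a debug sphere, then calls itself recursively.
; IsDead stops the brain, sight and actor tick after a short delay.
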(event OnPerceptionUpdated(AIPerception)
  (params (UpdatedActors :type Array%20of%20Actor%20Object%20References))
  ;[1 1 1] AI Perception and Targeting
  (for _array_element UpdatedActors
    (bind _info (Class|AIPerceptionComponent|GetActorsPerception (Variables|Default|GetAIPerception) _array_element))
    (CallFunction|CompleteSenses (.lastsensedstimuli _info))))

(event Custom|IsDead
  ;[1 1 1] Disable AI, Senses and Actor tick on Death
  (Utilities|FlowControl|Delay 1.0)
  (AI|Logic|StopLogic (Variables|Default|GetBrainComponent) "Dead")
  (Class|AIPerceptionComponent|SetSenseEnabled (Variables|Default|GetAIPerception) "/Script/AIModule.AISense_Sight" false)
  (Actor|Tick|SetActorTickEnabled false))

(event Custom|Configure%20AI%20Behaviour%20Tree%20and%20Senses
  ;[1 1 1] Add Behaviour Tree and set AI variables
  (AI|RunBehaviorTree "/Game/MyContent/AI/NPC/BehaviourTree/MasterNPC_BT.MasterNPC_BT")
  (bind _asmaster_npc (Utilities|Casting|CastToMasterNPC (Pawn|GetControlledPawn)))
  (bind _output_get (Variables|Default|SetMyPawn _asmaster_npc))
  (AI|Components|Blackboard|SetValueasObject (Variables|Default|GetBlackboard) (Utilities|Name|MakeLiteralName "SelfActor") _output_get)
  (bind _output_get_2 (Variables|Default|SetEnemy (Game|GetPlayerCharacter 0)))
  (AI|Components|Blackboard|SetValueasObject (Variables|Default|GetBlackboard) (Utilities|Name|MakeLiteralName "Enemy") _output_get_2))

(event EventBeginPlay
  ;[1 1 1] Initialise and Configure Behaviour Tree on Start
  (CallFunction|ConfigureAIBehaviourTreeandSenses))

(fn ConstructionScript)

(fn CompleteSenses
  (params (Stimulus :type Array%20of%20AI%20Stimulus%20Structures))
  (bind _enemy (Variables|Default|GetEnemy))
  (bind _returnvalue (Transformation|GetActorLocation _enemy))
  (for (_array_element _array_index) Stimulus
    (LocalVariables|SetLocalSense _array_element)
    (switch int _array_index
      (:0
        (bind _info (Class|AIPerceptionComponent|GetActorsPerception (Variables|Default|GetAIPerception)))
        (AI|Components|Blackboard|SetValueasBool (AI|GetBlackboard 0) (Utilities|Name|MakeLiteralName "CanSeePlayer") (.bsuccessfullysensed (LocalVariables|GetLocalSense)))
        (Utilities|IsValid _enemy
          (:Is%20Valid
            (AI|Components|Blackboard|SetValueasVector (Variables|Default|GetBlackboard) (Utilities|Name|MakeLiteralName "LastSeenLocation") _returnvalue)
            (Rendering|Debug|DrawDebugSphere _returnvalue 1e+02 12 "(R=1.000000,G=1.000000,B=1.000000,A=1.000000)" 5.0)
            (CallFunction|CompleteSenses (.LastSensedStimuli (Utilities|Struct|BreakActorPerceptionBlueprintInfo _info)))))))))